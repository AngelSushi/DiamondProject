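; BP_DoorToOpenPressurePlate is a door that opens and closes through reward and cancel events, intended for a pressure plate puzzle.
; RewardFunction plays the DoorOpening timeline, and CancelRewardFunction reverses it, each printing a debug message.
; The timeline's height value sets the door's relative location directly along the axis chosen by DoorAxis, with Z used for None.
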(event `self.RewardFunction`
  (bind _door (`self.door`))
  (`KismetSystemLibrary.PrintString` "Active True")
  (bind (_direction _heightfordoor) (`Timeline|DoorOpening` :!label _label)
    (:`Update`
      (switch `EAxis` (`self.DoorAxis`)
        (:`None`
          (`SceneComponent.K2_SetRelativeLocation` (`self.door`) (`KismetMathLibrary.MakeVector` 0.0 0.0 _heightfordoor) false false :!label _label_2))
        (:`X`
          (`SceneComponent.K2_SetRelativeLocation` _door (`KismetMathLibrary.MakeVector` _heightfordoor) false false))
        (:`Y`
          (`SceneComponent.K2_SetRelativeLocation` _door (`KismetMathLibrary.MakeVector` 0.0 _heightfordoor) false false))
        (:`Z`
          (goto _label_2))))))

(event `self.CancelRewardFunction`
  (`KismetSystemLibrary.PrintString` "Cancel Door" true true (struct :`R` 0.092799 :`G` 0.015615 :`B` 0.166667 :`A` 1.0) 10.0)
  (goto _label :!via `Reverse`))

(fn `UserConstructionScript`)