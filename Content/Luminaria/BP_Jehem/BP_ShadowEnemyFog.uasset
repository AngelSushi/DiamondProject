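; Shadow fog enemy character that makes a single pass toward the player and disappears.
; On BeginPlay it sets its walk speed, then uses AI MoveTo toward a fixed point twice as far as the player's starting position, overshooting rather than tracking.
; It destroys itself on reaching that point, or when its capsule hits the player, where it only prints a French game-over message.
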(event `self.ReceiveBeginPlay`
  (bind _returnvalue (`self.K2_GetActorLocation` self))
  (set `CharacterMovementComponent.MaxWalkSpeed` (`self.EnemySpeed`) (`self.CharacterMovement`))
  (`self.GoToTarget` (+ _returnvalue (* (- (`self.K2_GetActorLocation` (`GameplayStatics.GetPlayerCharacter` 0)) _returnvalue) 2.0))))

(event `GoToTarget`
  (params (TargetLocation :type "Vector Structure"))
  (`|AIMoveTo` self TargetLocation null
    (:`OnSuccess`
      (`self.K2_DestroyActor` self))))

(event `self.CapsuleComponent.OnComponentHit`
  (params (HitComponent :type "PrimitiveComponent Object Reference") (OtherActor :type "Actor Object Reference") (OtherComp :type "PrimitiveComponent Object Reference") (NormalImpulse :type "Vector Structure") (Hit :type "HitResult Structure (by ref)"))
  (if (== OtherActor (`GameplayStatics.GetPlayerCharacter` 0))
    (`KismetSystemLibrary.PrintString` "Tu perd la game mon grand garçon")
    (`self.K2_DestroyActor` self)))

(fn `UserConstructionScript`)