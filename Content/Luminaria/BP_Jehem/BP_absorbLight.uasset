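; BP_absorbLight is an actor that drains the light energy of the top-down player character when they enter its box.
; The first overlap with BP_TopDownCharacter subtracts Damage from its LightEnergy, with IsAbsorb guarding against repeat triggers.
; The AbsorbTime timeline then animates the point light's color, and the actor destroys itself when the timeline finishes.
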(event `self.Box.OnComponentBeginOverlap`
  (params (OverlappedComponent :type "PrimitiveComponent Object Reference") (OtherActor :type "Actor Object Reference") (OtherComp :type "PrimitiveComponent Object Reference") (OtherBodyIndex :type Integer) (bFromSweep :type Boolean) (SweepResult :type "HitResult Structure (by ref)"))
  (if (not (`self.isAbsorb`))
    (bind _asbp_top_down_character (cast `/Game/TopDown/Blueprints/BP_TopDownCharacter` OtherActor))
    (if (== OtherActor _asbp_top_down_character)
      (set `self.isAbsorb` true)
      (set `/Game/TopDown/Blueprints/BP_TopDownCharacter.lightEnergy` (- (`/Game/TopDown/Blueprints/BP_TopDownCharacter.lightEnergy` _asbp_top_down_character) (`self.damage`)) _asbp_top_down_character)
      (bind (_direction _newtrack_1) (`Timeline|AbsorbTime`)
        (:`Update`
          (`LightComponent.SetLightColor` (`self.PointLight`) _newtrack_1 true))
        (:`Finished`
          (`self.K2_DestroyActor`))))))

(fn `UserConstructionScript`)