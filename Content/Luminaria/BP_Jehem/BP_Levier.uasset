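; BP_Levier is a lever that the electric player (Pc_PlayerElectric) toggles to switch an activator on or off.
; A box overlap caches that controller and sets an in-zone flag, cleared when any DiamondProjectCharacter leaves.
; Tick polls the controller's IsInteracting without debouncing, flipping the state on each frame it is true.
; Each flip sets the activator, plays an on/off sound event, switches the point light and drives a timeline that slides the lever vertically.
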(event `self.Box.OnComponentBeginOverlap`
  (params (OverlappedComponent :type "PrimitiveComponent Object Reference") (OtherActor :type "Actor Object Reference") (OtherComp :type "PrimitiveComponent Object Reference") (OtherBodyIndex :type Integer) (bFromSweep :type Boolean) (SweepResult :type "HitResult Structure (by ref)"))
  (bind _asdiamond_project_character (cast `DiamondProjectCharacter` OtherActor))
  (bind _aspc_player_electric (cast `/Game/Luminaria/Config/Pc_PlayerElectric` (`Pawn.GetController` _asdiamond_project_character)))
  (set `self.isInZone` true))

(event `self.ReceiveTick`
  (params (DeltaSeconds :type "Float (single-precision)"))
  (bind _returnvalue (`self.K2_GetActorLocation`))
  (bind _pointlight (`self.PointLight`))
  (if (`self.isInZone`)
    (if (`/Game/Luminaria/Config/Pc_PlayerElectric.isInteracting` (stale `self.Box.OnComponentBeginOverlap` _aspc_player_electric))
      (if (`self.isLevierOn`)
        (`self.SetActivatorActivate` false)
        (set `self.isLevierOn` false)
        ;[0 0 0] [SD] GPE Lever Off
        (`FMODBlueprintStatics.PlayEventAtLocation` "/Game/FMOD/Events/SFX/GPE/GPE_Lever_Off.GPE_Lever_Off" (`KismetMathLibrary.Conv_VectorToTransform` _returnvalue))
        (`LightComponent.SetIntensity` _pointlight 0.0)
        (bind (_direction _levier) (`Timeline|PushLevier` :!via `Reverse` :!label _label)
          (:`Update`
            (`SceneComponent.K2_SetRelativeLocation` (`self.levier`) (`KismetMathLibrary.MakeVector` 0.0 0.0 (`KismetMathLibrary.Lerp` 60.0 10.0 _levier)) false false)))
        (else
          (`self.SetActivatorActivate` true)
          (set `self.isLevierOn` true)
          ;[0 0 0] [SD] GPE Lever On
          (`FMODBlueprintStatics.PlayEventAtLocation` "/Game/FMOD/Events/SFX/GPE/GPE_Lever_On.GPE_Lever_On" (`KismetMathLibrary.Conv_VectorToTransform` _returnvalue))
          (`LightComponent.SetIntensity` _pointlight 10000.0)
          (goto _label))))))

(event `self.Box.OnComponentEndOverlap`
  (params (OverlappedComponent :type "PrimitiveComponent Object Reference") (OtherActor :type "Actor Object Reference") (OtherComp :type "PrimitiveComponent Object Reference") (OtherBodyIndex :type Integer))
  (cast `DiamondProjectCharacter` OtherActor)
  (set `self.isInZone` false))

(fn `UserConstructionScript`)