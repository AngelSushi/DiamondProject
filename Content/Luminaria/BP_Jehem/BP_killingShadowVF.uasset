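; Moving killing-shadow hazard that waits for the level's BP_KillingShadowBegin actor to set CanStart.
; While active, it enables death collision and Niagara, moving at constant Speed toward its start location plus MoveToPos.
; Reaching the target's Y clears CanStart, disables collision and effect, and permanently ends the phase.
; Overlapping DiamondProjectCharacter prints a debug death message, shuts the shadow off and resets it to its start for another run.
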(event `self.ReceiveBeginPlay`
  (bind _deathcomponent (`self.DeathComponent`))
  (set `self.collisionToKill` (`PrimitiveComponent.GetCollisionEnabled` _deathcomponent))
  (`PrimitiveComponent.SetCollisionEnabled` _deathcomponent "NoCollision")
  (set `self.StartPos` (`self.K2_GetActorLocation` self))
  (set `self.targetPos` (+ (`self.K2_GetActorLocation`) (`self.moveToPos`)))
  (bind _returnvalue (`GameplayStatics.GetActorOfClass` "/Game/Luminaria/BP_Jehem/BP_KillingShadowBegin.BP_KillingShadowBegin_C"))
  (set `self.ref` _returnvalue))

(event `self.ReceiveTick`
  (params (DeltaSeconds :type "Float (single-precision)"))
  (bind _returnvalue (`self.K2_GetActorLocation`))
  (bind (_returnvalue_x _returnvalue_y) (`KismetMathLibrary.BreakVector` (`self.K2_GetActorLocation`)))
  (bind (_targetpos_x _targetpos_y) (`KismetMathLibrary.BreakVector` (`self.targetPos`)))
  (bind (_returnvalue_x_2 _returnvalue_y_2 _returnvalue_z) (`KismetMathLibrary.BreakVector` (`KismetMathLibrary.Normal` (- (`self.targetPos`) _returnvalue))))
  (if (`/Game/Luminaria/BP_Jehem/BP_KillingShadowBegin.canStart` (`self.ref`))
    (if (not (`self.shadowPhaseDone`))
      (`PrimitiveComponent.SetCollisionEnabled` (`self.DeathComponent`) (`self.collisionToKill`))
      (if (not (`self.shadowPhaseDone`))
        (`ActorComponent.Activate` (`self.Niagara`) false)
        (`self.K2_SetActorLocation` (+ _returnvalue (* (* (`KismetMathLibrary.MakeVector` _returnvalue_x_2 _returnvalue_y_2 _returnvalue_z) (`self.speed`)) DeltaSeconds)))
        (if (>= _returnvalue_y _targetpos_y)
          (`ActorComponent.Deactivate` (`self.Niagara`))
          (set `/Game/Luminaria/BP_Jehem/BP_KillingShadowBegin.canStart` false (`self.ref`))
          (`PrimitiveComponent.SetCollisionEnabled` (`self.DeathComponent`) "NoCollision")
          (set `self.shadowPhaseDone` true))))))

(event `self.DeathComponent.OnComponentBeginOverlap`
  (params (OverlappedComponent :type "PrimitiveComponent Object Reference") (OtherActor :type "Actor Object Reference") (OtherComp :type "PrimitiveComponent Object Reference") (OtherBodyIndex :type Integer) (bFromSweep :type Boolean) (SweepResult :type "HitResult Structure (by ref)"))
  (if (`/Game/Luminaria/BP_Jehem/BP_KillingShadowBegin.canStart` (`self.ref`))
    (cast `DiamondProjectCharacter` OtherActor)
    (`KismetSystemLibrary.PrintString` "mort moRT MORT")
    (`ActorComponent.Deactivate` (`self.Niagara`))
    (set `/Game/Luminaria/BP_Jehem/BP_KillingShadowBegin.canStart` false (`self.ref`))
    (`PrimitiveComponent.SetCollisionEnabled` (`self.DeathComponent`) "NoCollision")
    (`self.K2_SetActorLocation` (`self.StartPos`))))

(fn `UserConstructionScript`)