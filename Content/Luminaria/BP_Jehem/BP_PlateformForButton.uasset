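; Moving platform that travels between its start position and an offset target, driven by reward events or a linked button.
; BeginPlay caches both endpoints, and RewardFunction and CancelRewardFunction toggle IsMoving.
; While IsMoving, Tick either ping-pongs between endpoints or steps toward the target at Speed.
; Otherwise, a valid RefButtonPlateform sends it toward the target when active and back to start when inactive, with no arrival clamp.
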(event `self.ReceiveBeginPlay`
  (set `self.StartPos` (`self.K2_GetActorLocation` self))
  (set `self.targetPos` (+ (`self.K2_GetActorLocation`) (`self.moveToPos`))))

(event `self.ReceiveTick`
  (params (DeltaSeconds :type "Float (single-precision)"))
  (bind _returnvalue (`self.K2_GetActorLocation`))
  (bind _returnvalue_2 (`self.K2_GetActorLocation`))
  (bind _refbuttonplateform (`self.refButtonPlateform`))
  (bind (_returnvalue_x _returnvalue_y _returnvalue_z) (`KismetMathLibrary.BreakVector` (`KismetMathLibrary.Normal` (- (`self.targetPos`) _returnvalue))))
  (bind (_returnvalue_x_2 _returnvalue_y_2 _returnvalue_z_2) (`KismetMathLibrary.BreakVector` (`KismetMathLibrary.Normal` (- (`self.StartPos`) _returnvalue_2))))
  (if (`self.IsMoving`)
    (if (`self.IsPingPong`)
      (bind _output_get (set `self.Timer` (+ (* DeltaSeconds (`self.speed`)) (`self.Timer`))))
      (`self.K2_SetActorLocation` (`MathUtilities.PingPongVec` _output_get (`self.targetPos`) (`self.StartPos`)))
      (else
        (`self.K2_SetActorLocation` (+ _returnvalue (* (* (`KismetMathLibrary.MakeVector` _returnvalue_x _returnvalue_y _returnvalue_z) (`self.speed`)) DeltaSeconds)) :!label _label)))
    (else
      (`/Engine/EditorBlueprintResources/StandardMacros.IsValid` _refbuttonplateform
        (:`Is Valid`
          (if (`/Game/Luminaria/BP_Jehem/BP_PlateformButton.isActive` _refbuttonplateform)
            (goto _label)
            (else
              (`self.K2_SetActorLocation` (+ _returnvalue_2 (* (* (`KismetMathLibrary.MakeVector` _returnvalue_x_2 _returnvalue_y_2 _returnvalue_z_2) (`self.speed`)) DeltaSeconds))))))))))

(event `self.RewardFunction`
  (`KismetSystemLibrary.PrintString` "Reward Function")
  (set `self.IsMoving` true))

(event `self.CancelRewardFunction`
  (`KismetSystemLibrary.PrintString` "Cancel Reward Function")
  (set `self.IsMoving` false))

(fn `UserConstructionScript`)