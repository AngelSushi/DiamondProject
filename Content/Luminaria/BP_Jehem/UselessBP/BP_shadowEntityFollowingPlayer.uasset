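; Shadow entity actor, named as a player follower, that slides along the world Y axis toward a stored target point.
; Until IsTargetReached is set, Tick moves it without sweep by the Y component of the normalized direction, scaled by Speed and delta time.
; Nothing here sets the target or flag, and the player-location math is unconnected.
; Sphere overlap with the player only prints a debug string.
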(event `self.ReceiveTick`
  (params (DeltaSeconds :type "Float (single-precision)"))
  (bind _returnvalue (`self.K2_GetActorLocation`))
  (bind (_returnvalue_x _returnvalue_y) (`KismetMathLibrary.BreakVector` (`KismetMathLibrary.Normal` (- (`self.targetToReach`) _returnvalue) 0.0)))
  (if (not (`self.isTargetReached`))
    (`self.K2_SetActorLocation` (+ _returnvalue (* (* (`KismetMathLibrary.MakeVector` 0.0 _returnvalue_y) (`self.speed`)) DeltaSeconds)))))

(event `self.Sphere.OnComponentBeginOverlap`
  (params (OverlappedComponent :type "PrimitiveComponent Object Reference") (OtherActor :type "Actor Object Reference") (OtherComp :type "PrimitiveComponent Object Reference") (OtherBodyIndex :type Integer) (bFromSweep :type Boolean) (SweepResult :type "HitResult Structure (by ref)"))
  (bind _returnvalue (== OtherActor (`GameplayStatics.GetPlayerCharacter` 0)))
  (if _returnvalue
    (`KismetSystemLibrary.PrintString` (`KismetStringLibrary.Conv_BoolToString` _returnvalue))))

(fn `UserConstructionScript`)