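; BP_FogEnemyV2 is a fog enemy actor that charges in a straight line toward where the player stood when it spawned.
; BeginPlay sets a target twice the distance to the player and sets its yaw from the player direction with a 90-degree offset.
; Tick moves it at Speed without sweeping while IsTargetReached is false, a flag this graph never sets.
; Capsule overlap with the player prints a debug string and destroys the enemy.
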(event `self.ReceiveBeginPlay`
  (bind _returnvalue (`self.K2_GetActorLocation` self))
  (bind (_returnvalue_roll _returnvalue_pitch _returnvalue_yaw) (`KismetMathLibrary.BreakRotator` (`KismetMathLibrary.MakeRotFromX` (- (`self.K2_GetActorLocation`) (`self.K2_GetActorLocation` (`GameplayStatics.GetPlayerPawn` 0))))))
  (set `self.targetToReach` (+ _returnvalue (* (- (`self.K2_GetActorLocation` (`GameplayStatics.GetPlayerCharacter` 0)) _returnvalue) 2.0)))
  ;[1 1 1] Rotation de l'enemy
  (`self.K2_SetActorRotation` (`KismetMathLibrary.MakeRotator` 0.0 0.0 (+ _returnvalue_yaw 90.0))))

(event `self.ReceiveTick`
  (params (DeltaSeconds :type "Float (single-precision)"))
  (bind _returnvalue (`self.K2_GetActorLocation`))
  (bind (_returnvalue_x _returnvalue_y _returnvalue_z) (`KismetMathLibrary.BreakVector` (`KismetMathLibrary.Normal` (- (`self.targetToReach`) _returnvalue) 0.0)))
  (if (not (`self.isTargetReached`))
    (`self.K2_SetActorLocation` (+ _returnvalue (* (* (`KismetMathLibrary.MakeVector` _returnvalue_x _returnvalue_y _returnvalue_z) (`self.speed`)) DeltaSeconds)))))

(event `self.Capsule.OnComponentBeginOverlap`
  (params (OverlappedComponent :type "PrimitiveComponent Object Reference") (OtherActor :type "Actor Object Reference") (OtherComp :type "PrimitiveComponent Object Reference") (OtherBodyIndex :type Integer) (bFromSweep :type Boolean) (SweepResult :type "HitResult Structure (by ref)"))
  (bind _returnvalue (== OtherActor (`GameplayStatics.GetPlayerCharacter` 0)))
  (if _returnvalue
    (`KismetSystemLibrary.PrintString` (`KismetStringLibrary.Conv_BoolToString` _returnvalue))
    (`self.K2_DestroyActor`)))

(fn `UserConstructionScript`)