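; Door actor that opens once enough pressure plates or switches are active at the same time.
; Activation and deactivation events adjust a counter and compare it to a required count.
; Meeting the count plays a timeline, and falling short reverses it.
; The timeline's height curve drives the door's relative location along a selectable axis.
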(event `SwitcheActivated`
  (`/Engine/EditorBlueprintResources/StandardMacros.IncrementInt` (`self.pressurePlateActive`)
    (:`  `
      (if (>= (`self.pressurePlateActive`) (`self.pressurePlateNeeded`))
        (bind (_direction _heightfordoor) (`Timeline|DoorOpening` :!label _label)
          (:`Update`
            (switch `EAxis` (`self.DoorAxis`)
              (:`X`
                (`SceneComponent.K2_SetRelativeLocation` (`self.door`) (`KismetMathLibrary.MakeVector` _heightfordoor) false false))
              (:`Y`
                (`SceneComponent.K2_SetRelativeLocation` (`self.door`) (`KismetMathLibrary.MakeVector` 0.0 _heightfordoor) false false))
              (:`Z`
                (`SceneComponent.K2_SetRelativeLocation` (`self.door`) (`KismetMathLibrary.MakeVector` 0.0 0.0 _heightfordoor) false false)))))
        (else
          (goto _label :!via `Reverse`))))))

(event `switchDesactivated`
  (`/Engine/EditorBlueprintResources/StandardMacros.DecrementInt` (`self.pressurePlateActive`)
    (:`  `
      (if (>= (`self.pressurePlateActive`) (`self.pressurePlateNeeded`))
        (goto _label)
        (else
          (goto _label :!via `Reverse`))))))

(fn `UserConstructionScript`)