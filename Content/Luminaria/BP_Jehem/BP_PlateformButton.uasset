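; Pressure plate button that switches its activator state when a movable box, or a player with enough LightValue, stands on it.
; Box overlaps track an occupant count and box presence, checking the player's light only on entry; the button releases when the count empties.
; Tick also releases it if the stored player's light drops below the threshold without a box present.
; Press and release play sounds and move the button through a reversible timeline.
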(event `self.ReceiveTick`
  (params (DeltaSeconds :type "Float (single-precision)"))
  (if (`self.isActive`)
    (if (`self.isBoxOnButton`)
      _
      (elif (not (>= (`/Game/Luminaria/Config/Pc_PlayerElectric.LightValue` (stale `self.Box.OnComponentBeginOverlap` _aspc_player_electric)) (`self.lightValueNeeded`)))
        (`self.buttonRelease`)))))

(event `self.Box.OnComponentBeginOverlap`
  (params (OverlappedComponent :type "PrimitiveComponent Object Reference") (OtherActor :type "Actor Object Reference") (OtherComp :type "PrimitiveComponent Object Reference") (OtherBodyIndex :type Integer) (bFromSweep :type Boolean) (SweepResult :type "HitResult Structure (by ref)"))
  (bind _isactive (`self.isActive`))
  (bind _asdiamond_project_character (cast `DiamondProjectCharacter` OtherActor)
    (:`then`
      (bind _aspc_player_electric (cast `/Game/Luminaria/Config/Pc_PlayerElectric` (`Pawn.GetController` _asdiamond_project_character)))
      (set `self.nbPlayerOnButton` (+ (`self.nbPlayerOnButton`) 1))
      (if _isactive
        _
        (elif (>= (`/Game/Luminaria/Config/Pc_PlayerElectric.LightValue` _aspc_player_electric) (`self.lightValueNeeded`))
          (set `self.goodLightValue` true)
          (`self.ButtonPress`)
          (else
            (set `self.goodLightValue` false)))))
    (:`CastFailed`
      (cast `/Game/Luminaria/BP_Jehem/BP_MovableObject` OtherActor)
      (set `self.nbPlayerOnButton` (+ (`self.nbPlayerOnButton`) 1))
      (set `self.isBoxOnButton` true)
      (if (not _isactive)
        (`self.ButtonPress`)))))

(event `ButtonPress`
  (`self.SetActivatorActivate` true)
  (`GameplayStatics.PlaySoundAtLocation` "/Engine/VREditor/Sounds/UI/Click_on_Button.Click_on_Button" (`self.K2_GetActorLocation`) (struct) 1.0 1.0 0.0 null null null null)
  (set `self.isActive` true)
  (bind (_direction _buttonpressed) (`Timeline|ButtonPression` :!label _label)
    (:`Update`
      (`SceneComponent.K2_SetRelativeLocation` (`self.button`) (`KismetMathLibrary.MakeVector` 0.0 0.0 (`KismetMathLibrary.Lerp` 5.0 -5.0 _buttonpressed)) false false))))

(event `self.Box.OnComponentEndOverlap`
  (params (OverlappedComponent :type "PrimitiveComponent Object Reference") (OtherActor :type "Actor Object Reference") (OtherComp :type "PrimitiveComponent Object Reference") (OtherBodyIndex :type Integer))
  (cast `DiamondProjectCharacter` OtherActor
    (:`then`
      (set `self.nbPlayerOnButton` (- (`self.nbPlayerOnButton`) 1)))
    (:`CastFailed`
      (cast `/Game/Luminaria/BP_Jehem/BP_MovableObject` OtherActor)
      (set `self.isBoxOnButton` false)
      (set `self.nbPlayerOnButton` (- (`self.nbPlayerOnButton`) 1))))
  (if (`self.isActive`)
    (if (not (> (`self.nbPlayerOnButton`) 0))
      (`self.buttonRelease`))))

(event `buttonRelease`
  (`self.SetActivatorActivate` false)
  (`GameplayStatics.PlaySoundAtLocation` "/Engine/VREditor/Sounds/UI/Camera_Shutter.Camera_Shutter" (`self.K2_GetActorLocation`) (struct) 1.0 1.0 0.0 null null null null)
  (set `self.isActive` false)
  (goto _label :!via `Reverse`))

(fn `UserConstructionScript`)