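; Movable cube that the top-down character can push or pull when the player's light value meets a required threshold.
; The Forward overlap caches the character and controller and toggles pushing permission, which also governs CanFlip on the DiamondProjectPlayerController.
; While the push button is held in the zone, Tick slows walking and reads move input to choose push or pull.
; Speeddirection then slides the cube along its right vector with VInterpTo, without sweep.
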(event `self.ReceiveBeginPlay`
  (bind _returnvalue (`GameplayStatics.GetActorOfClass` "/Script/DiamondProject.DiamondProjectPlayerController"))
  (set `self.refDiamonController` _returnvalue))

(event `self.ReceiveTick`
  (params (DeltaSeconds :type "Float (single-precision)"))
  (bind _as_bp_top_down_character (`self.As BP Top Down Character`))
  (bind _cubespeed (`self.cubeSpeed`))
  (bind _move_value (`/Game/TopDown/Blueprints/BP_TopDownCharacter.Move value` (`self.As BP Top Down Character`)))
  (bind _charactermovement (`Character.CharacterMovement` _as_bp_top_down_character))
  (`KismetSystemLibrary.PrintString` (`KismetStringLibrary.Conv_BoolToString` (`self.isPushing`)))
  (`KismetSystemLibrary.PrintString` (`KismetStringLibrary.Conv_BoolToString` (`self.isPulling`)))
  (if (`KismetSystemLibrary.IsValid` _as_bp_top_down_character)
    (if (`/Game/TopDown/Blueprints/BP_TopDownCharacter.buttonPushPressed` _as_bp_top_down_character)
      (if (`self.isInZone`)
        (if (>= (`/Game/Luminaria/Config/PC_Player.LightValue` (stale `self.forward.OnComponentBeginOverlap` _aspc_player)) (`self.lightValueNeeded`))
          (set `CharacterMovementComponent.MaxWalkSpeed` 60.0 _charactermovement)
          (if (`/Game/TopDown/Blueprints/BP_TopDownCharacter.canPush` _as_bp_top_down_character)
            (if (== _move_value (0.0 0.0))
              _
              (elif (== _move_value (1.0 0.0))
                (set `self.isPushing` true)
                (set `self.isPulling` false)
                (`self.Speed/direction` true (* _cubespeed -1.0))
                (else
                  (set `self.isPulling` true)
                  (set `self.isPushing` false)
                  (`self.Speed/direction` true _cubespeed)))))
          (else
            (`self.StopPushing` :!label _label)
            (set `CharacterMovementComponent.MaxWalkSpeed` 600.0 _charactermovement :!label _label_2)))
        (else
          (goto _label)))
      (else
        (goto _label_2)))))

(event `self.forward.OnComponentBeginOverlap`
  (params (OverlappedComponent :type "PrimitiveComponent Object Reference") (OtherActor :type "Actor Object Reference") (OtherComp :type "PrimitiveComponent Object Reference") (OtherBodyIndex :type Integer) (bFromSweep :type Boolean) (SweepResult :type "HitResult Structure (by ref)"))
  (bind _asbp_top_down_character (cast `/Game/TopDown/Blueprints/BP_TopDownCharacter` OtherActor))
  (set `self.As BP Top Down Character` _asbp_top_down_character)
  (bind _aspc_player (cast `/Game/Luminaria/Config/PC_Player` (`Pawn.GetController` _asbp_top_down_character)))
  (bind _output_get (set `self.isInZone` true))
  (`KismetSystemLibrary.PrintString` (`KismetStringLibrary.Conv_BoolToString` _output_get))
  (if (>= (`/Game/Luminaria/Config/PC_Player.LightValue` _aspc_player) (`self.lightValueNeeded`))
    (set `self.goodLightVallue` true)
    (`self.startPushing`)
    (else
      (set `self.goodLightVallue` false)
      (`self.StopPushing`))))

(event `self.forward.OnComponentEndOverlap`
  (params (OverlappedComponent :type "PrimitiveComponent Object Reference") (OtherActor :type "Actor Object Reference") (OtherComp :type "PrimitiveComponent Object Reference") (OtherBodyIndex :type Integer))
  (bind _asbp_top_down_character (cast `/Game/TopDown/Blueprints/BP_TopDownCharacter` OtherActor))
  (cast `/Game/Luminaria/Config/PC_Player` (`Pawn.GetController` _asbp_top_down_character))
  (set `self.isInZone` false)
  (if (not (>= (`/Game/Luminaria/Config/PC_Player.LightValue` (stale `self.forward.OnComponentBeginOverlap` _aspc_player)) (`self.lightValueNeeded`)))
    (`self.StopPushing`)))

(event `startPushing`
  (bind _as_bp_top_down_character (`self.As BP Top Down Character`))
  (set `/Game/TopDown/Blueprints/BP_TopDownCharacter.canPush` true _as_bp_top_down_character)
  (if (`/Game/TopDown/Blueprints/BP_TopDownCharacter.buttonPushPressed` _as_bp_top_down_character)
    (set `DiamondProjectPlayerController.bCanFlip` false (`self.refDiamonController`))))

(event `StopPushing`
  (set `/Game/TopDown/Blueprints/BP_TopDownCharacter.canPush` false (`self.As BP Top Down Character`))
  (set `DiamondProjectPlayerController.bCanFlip` true (`self.refDiamonController`)))

(fn `UserConstructionScript`)