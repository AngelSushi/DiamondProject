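; Moving ground platform Blueprint that, as wired, only handles its sound and mechanism bindings.
; BeginPlay plays the FMOD platform-move event once on the FMODAudio component and binds to the mechanism dispatcher's on/off events.
; Those handlers and StartPlateform/StopPlateform are empty.
; The waypoint-to-control-point path setup, auto-activation and movement start/stop toggling sit in disconnected nodes that never run.
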(event `self.ReceiveBeginPlay`
  (bind _returnvalue (subsystem `MecanismEventsDispatcher`))
  ;[0 0 0] [SD] GPE Platform
  (`/Engine/EditorBlueprintResources/StandardMacros.DoOnce` false
    (:`Completed`
      (`FMODBlueprintStatics.PlayEventAttached` "/Game/FMOD/Events/SFX/GPE/GPE_PlatformMove.GPE_PlatformMove" (`self.FMODAudio`) "None" (0.0 0.0 0.0) "KeepRelativeOffset")
      (add `MecanismEventsDispatcher.OnMecanismOn` _returnvalue (delegate `OnMecanismOn_Event_0`))
      (add `MecanismEventsDispatcher.OnMecanismOff` _returnvalue (delegate `OnMecanismOff_Event_0`)))))

(event `StartPlateform`)

(event `StopPlateform`)

(event `OnMecanismOn_Event_0`
  (params (TargetMecanism :type "Mecanism Object Reference")))

(event `OnMecanismOff_Event_0`
  (params (TargetMecanism :type "Mecanism Object Reference")))

(fn `UserConstructionScript`)