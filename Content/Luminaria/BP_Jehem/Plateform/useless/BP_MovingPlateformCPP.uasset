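; Moving platform Blueprint that follows a path built from component positions through an InterpToMovement component.
; The construction script adds a relative origin control point, then loops over GetComponentPositions to append each position as a relative point.
; It indexes the positions with a separate MoveToPoseElement counter, incremented on each pass, instead of the loop index.
; The event graph holds only disabled placeholder events, and MoveToPos is unused.
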(fn `UserConstructionScript`
  (bind _returnvalue (`self.GetComponentPositions`))
  (bind _returnvalue_2 (`KismetArrayLibrary.Array_Length` _returnvalue))
  (`InterpToMovementComponent.AddControlPointPosition` (`self.InterpToMovement`) (0.0 0.0 0.0) true)
  (if (> _returnvalue_2 0)
    (for _ (range (+ _returnvalue_2 1))
      (`InterpToMovementComponent.AddControlPointPosition` (`self.InterpToMovement`) (`|GetArrayItem` _returnvalue (`self.MoveToPoseElement`)) true)
      (set `self.MoveToPoseElement` (+ (`self.MoveToPoseElement`) 1)))))