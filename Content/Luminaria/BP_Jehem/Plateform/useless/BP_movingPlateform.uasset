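; Moving platform Blueprint that configures its InterpToMovement component with a path from a MoveToPos array of relative positions.
; The construction script adds a control point at the relative origin, then loops over the array length, using the MoveToPoseElement counter to add each further point.
; It also prints the array length as debug output when the array is not empty.
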(fn `UserConstructionScript`
  (bind _movetopos (`self.moveToPos`))
  (bind _returnvalue (`KismetArrayLibrary.Array_Length` _movetopos))
  (`InterpToMovementComponent.AddControlPointPosition` (`self.InterpToMovement`) (0.0 0.0 0.0) true)
  (if (> _returnvalue 0)
    (`/Engine/EditorBlueprintResources/StandardMacros.IsValid` self
      (:`Is Valid`
        (`KismetSystemLibrary.PrintString` (`KismetStringLibrary.Conv_IntToString` _returnvalue))
        (for _ (range (+ _returnvalue 1))
          (`InterpToMovementComponent.AddControlPointPosition` (`self.InterpToMovement`) (`|GetArrayItem` _movetopos (`self.MoveToPoseElement`)) true)
          (set `self.MoveToPoseElement` (+ (`self.MoveToPoseElement`) 1)))))))