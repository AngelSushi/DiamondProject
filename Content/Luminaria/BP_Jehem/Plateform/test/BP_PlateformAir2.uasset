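; Moving platform Blueprint that travels along a path defined by placed waypoint actors.
; The construction script feeds waypoint world locations into an InterpToMovement component, sets its duration and enables auto-activation for auto platforms.
; StartPlateform and StopPlateform events resume and pause motion by toggling the component's tick, both leaving it active.
; BeginPlay attaches the FMOD platform-move sound once.
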(event `self.ReceiveBeginPlay`
  ;[0 0 0] [SD] GPE Platform
  (`/Engine/EditorBlueprintResources/StandardMacros.DoOnce` false
    (:`Completed`
      (`FMODBlueprintStatics.PlayEventAttached` "/Game/FMOD/Events/SFX/GPE/GPE_PlatformMove.GPE_PlatformMove" (`self.FMODAudio`) "None" (0.0 0.0 0.0) "KeepRelativeOffset"))))

(event `StartPlateform`
  (bind _interptomovement (`self.InterpToMovement`))
  (`ActorComponent.SetActive` _interptomovement true false)
  (`ActorComponent.SetComponentTickEnabled` _interptomovement true))

(event `StopPlateform`
  (bind _interptomovement (`self.InterpToMovement`))
  (`ActorComponent.SetActive` _interptomovement true false)
  (`ActorComponent.SetComponentTickEnabled` _interptomovement false))

(fn `UserConstructionScript`
  (bind _interptomovement (`self.InterpToMovement`))
  (for _array_element (`self.Waypoints`)
    (`InterpToMovementComponent.AddControlPointPosition` (`self.InterpToMovement`) (`self.K2_GetActorLocation` _array_element) false))
  (set `InterpToMovementComponent.Duration` (`self.duration`) _interptomovement)
  (if (`self.isAutoPlateform`)
    (`ActorComponent.SetAutoActivate` _interptomovement true)
    (else
      (`ActorComponent.SetAutoActivate` _interptomovement false))))