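; Spline audio actor that plays a looping FMOD tentacle event from the point on its spline nearest the player's view target.
; BeginPlay attaches the event to the FMOD component, then starts MoveAudio, which re-runs itself on a short delay.
; Each pass moves the audio component and a sphere to that closest spline point, raised slightly.
; Spline mesh construction and debug drawing code exist but are disconnected.
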(event `self.ReceiveBeginPlay`
  (`FMODBlueprintStatics.PlayEventAttached` "/Game/FMOD/Events/SFX/GPE/GPE_Tentacle_lp.GPE_Tentacle_lp" (`self.FMODAudio`) "None" (0.0 0.0 0.0) "KeepRelativeOffset")
  (`self.Move Audio`))

(event `Move Audio`
  (bind (_returnvalue_x _returnvalue_y _returnvalue_z) (`KismetMathLibrary.BreakVector` (`SplineComponent.FindLocationClosestToWorldLocation` (`self.Spline`) (`self.K2_GetActorLocation` (`Controller.GetViewTarget` (`GameplayStatics.GetPlayerController` 0))) "World")))
  (`SceneComponent.K2_SetWorldLocation` (`self.FMODAudio`) (`KismetMathLibrary.MakeVector` _returnvalue_x _returnvalue_y (+ _returnvalue_z 50.0)) false false)
  (`SceneComponent.K2_SetWorldLocation` (`self.Sphere`) (`KismetMathLibrary.MakeVector` _returnvalue_x _returnvalue_y (+ _returnvalue_z 50.0)) false false)
  (`KismetSystemLibrary.Delay` 0.05)
  (`self.Move Audio`))

(fn `UserConstructionScript`)