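; Test actor for the Luminaria camera system that currently has no effect in game.
; Each tick it checks whether the player's main camera is in an area with dynamic behavior, but the branch does nothing.
; Disconnected logic would place the actor at the player's X and the dynamic camera barycenter's Y and Z.
; An unused screen-to-world deprojection is also left in the graph.
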(event `self.ReceiveTick`
  (params (DeltaSeconds :type "Float (single-precision)"))
  (bind _returnvalue (`DiamondProjectCharacter.GetMainCamera` (`PlayerManager.GetOnePlayer` (subsystem `PlayerManager`))))
  (if (== (`CameraArea.AreaBehavior` (`LuminariaCamera.GetCurrentArea` _returnvalue)) (`KismetMathLibrary.Conv_ByteToInt` (enumliteral `ECameraBehavior` "DYNAMIC")))
    _))

(fn `UserConstructionScript`)