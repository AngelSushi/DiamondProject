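; Actor that switches an accessibility post-process on or off to match the IsAccessibility flag in GI_MainGameInstance.
; BeginPlay applies the flag to the PostProcessAccessibility component's Enabled state, and Tick polls the game instance to update it whenever the two differ.
; A debug T key flips the flag in the game instance, leaving Tick to apply the visual change.
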(event EventBeginPlay
  (bind _postprocessaccessibility (Variables|Default|GetPostProcessAccessibility))
  (bind _asgi_main_game_instance (Utilities|Casting|CastToGI_MainGameInstance (Game|GetGameInstance)))
  (if (Utilities|IsValid _postprocessaccessibility)
    (Variables|/Script/Engine.PostProcessVolume|SetbEnabled _postprocessaccessibility (Variables|/Game/Luminaria/Config/GI_MainGameInstance.GI_MainGameInstance_C|GetIsAccessibility _asgi_main_game_instance))))

(event EventTick
  (params (DeltaSeconds :type Float%20%28single-precision%29))
  (bind _postprocessaccessibility (Variables|Default|GetPostProcessAccessibility))
  (bind _asgi_main_game_instance (Utilities|Casting|CastToGI_MainGameInstance (Game|GetGameInstance)))
  (if (!= (Variables|/Game/Luminaria/Config/GI_MainGameInstance.GI_MainGameInstance_C|GetIsAccessibility _asgi_main_game_instance) (Variables|/Script/Engine.PostProcessVolume|GetbEnabled _postprocessaccessibility))
    (Variables|/Script/Engine.PostProcessVolume|SetbEnabled _postprocessaccessibility (Variables|/Game/Luminaria/Config/GI_MainGameInstance.GI_MainGameInstance_C|GetIsAccessibility _asgi_main_game_instance))))

(event Input|KeyboardEvents|DebugKeyT
  (params (Key :type Key%20Structure :default "None") (ActionValue :type Input%20Action%20Value%20Structure))
  (:Pressed
    (bind _asgi_main_game_instance (Utilities|Casting|CastToGI_MainGameInstance (Game|GetGameInstance)))
    (Variables|/Game/Luminaria/Config/GI_MainGameInstance.GI_MainGameInstance_C|SetIsAccessibility _asgi_main_game_instance (not (Variables|/Game/Luminaria/Config/GI_MainGameInstance.GI_MainGameInstance_C|GetIsAccessibility _asgi_main_game_instance)))))

(fn ConstructionScript)