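; BP_LDMaker builds a level layout from a JSON block-data file through ConstructLD.
; Each block spawns the class selected by its index from ActorsIndex, offset from the maker's location, with Y and Z swapped for position and scale.
; Activator and reward actors with a non-negative mechanism index are recorded in a map.
; ConstructMecanism then attempts to group them by that index, spawning Mecanism actors that receive them as activators or results.
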(fn `ConstructLD`
  (bind _mecanismactors (`self.MecanismActors`))
  ;[1 1 1] Check If Mecanism Needed
  ;;[1 1 1] Create Actor From BlockData
  ;;;[1 1 1] Get BlocksData From Json File
  (bind (_outjsonobject _returnvalue) (`JsonBlueprintFunctionLibrary.FromFile` (`self.LDFile`)))
  (if _returnvalue
    (bind (_outvalue _returnvalue_2) (`|GetJsonField` _outjsonobject "blocksDatas"))
    (`BlueprintMapLibrary.Map_Clear` (`self.MecanismActors`))
    (if _returnvalue_2
      (for _array_element _outvalue
        (bind _values (`BlueprintMapLibrary.Map_Values` (`self.ActorsIndex`)))
        (bind (__blockindex __mecanismindex __worldx __worldy __worldz __screenx __screeny __screenz __sizex __sizey __sizez) (break `/Game/Luminaria/LDs/BlockData` _array_element))
        (bind _returnvalue_3 (`|SpawnActorFromClass` (`|GetArrayItem` _values __blockindex) (`KismetMathLibrary.MakeTransform` (+ (`self.K2_GetActorLocation`) (`KismetMathLibrary.MakeVector` __worldx __worldz __worldy)) (`self.K2_GetActorRotation`) (`KismetMathLibrary.MakeVector` __sizex __sizez __sizey)) "Undefined" "MultiplyWithRoot" null null))
        (bind _asmecanism_activator (cast `MecanismActivator` _returnvalue_3)
          (:`then`
            (bind _returnvalue_4 (`KismetStringLibrary.Concat_StrStr` "Index de mécanisme" (`KismetStringLibrary.Conv_IntToString` __mecanismindex)))
            (`KismetSystemLibrary.PrintString` _returnvalue_4)
            (bind _returnvalue_5 (>= __mecanismindex 0))
            (if _returnvalue_5
              (`BlueprintMapLibrary.Map_Add` _mecanismactors _asmecanism_activator __mecanismindex)))
          (:`CastFailed`
            (bind _asmecanism_reward_actor (cast `MecanismRewardActor` _returnvalue_3))
            (`KismetSystemLibrary.PrintString` _returnvalue_4)
            (if _returnvalue_5
              (`BlueprintMapLibrary.Map_Add` _mecanismactors _asmecanism_reward_actor __mecanismindex)))))
      (`self.ConstructMecanism` (`self.MecanismActors`)))))

(fn `ConstructMecanism`
  (params (ActorsList :type "Map of Actor Object Reference to Integer"))
  (bind _values (`BlueprintMapLibrary.Map_Values` ActorsList))
  (for (_array_element _array_index) _values
    (bind _values_2 (`BlueprintMapLibrary.Map_Values` ActorsList))
    (bind _result (`/Engine/EditorBlueprintResources/StandardMacros.IncrementInt` _array_index)
      (:`  `
        (`KismetArrayLibrary.Array_Clear` (`self.ActorsInMecanism`))
        (for _index (range _result (+ (`KismetArrayLibrary.Array_Length` _values_2) 1))
          (bind _output (`|GetArrayItem` _values_2 _index))
          (if (== _array_element _output)
            (bind _keys (`BlueprintMapLibrary.Map_Keys` ActorsList))
            (bind _output_2 (`|GetArrayItem` _keys _output))
            (`KismetArrayLibrary.Array_Add` (`self.ActorsInMecanism`) _output_2)
            (`BlueprintMapLibrary.Map_Remove` ActorsList _output_2)))
        (if (> (`KismetArrayLibrary.Array_Length` (`self.ActorsInMecanism`)) 0)
          (bind _returnvalue (`|SpawnActorFromClass` "/Script/DiamondProject.Mecanism" (`KismetMathLibrary.MakeTransform` (0.0 0.0 0.0)) "Undefined" "MultiplyWithRoot" null null))
          (for _array_element_2 (`self.ActorsInMecanism`)
            (bind _asmecanism_activator (cast `MecanismActivator` _array_element_2)
              (:`then`
                (`KismetArrayLibrary.Array_Add` (`Mecanism.MecanismActivators` _returnvalue) _asmecanism_activator))
              (:`CastFailed`
                (bind _asmecanism_reward_actor (cast `MecanismRewardActor` _array_element_2))
                (`KismetArrayLibrary.Array_Add` (`Mecanism.MecanismResults` _returnvalue) _asmecanism_reward_actor)))))))))

(fn `UserConstructionScript`)