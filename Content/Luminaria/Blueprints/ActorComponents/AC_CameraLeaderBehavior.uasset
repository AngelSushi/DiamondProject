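; Actor component meant to make its owning actor, by its name a camera, follow a leader character.
; BeginPlay picks a random DiamondProjectCharacter and stores it as Leader.
; The follow logic, which matches the leader's X and raised Z while keeping the owner's Y, is disconnected from the empty Tick event, so it never runs.
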(event `self.ReceiveBeginPlay`
  (`parent.ReceiveBeginPlay`)
  (bind _outactors (`GameplayStatics.GetAllActorsOfClass` "/Script/DiamondProject.DiamondProjectCharacter"))
  (set `self.leader` (`KismetArrayLibrary.Array_Random` _outactors)))

(event `self.ReceiveTick`
  (params (DeltaSeconds :type "Float (single-precision)")))