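; Actor component intended for dynamic camera behavior based on the distance between two players, currently unfinished.
; One second after BeginPlay it caches all DiamondProjectCharacter actors.
; Each tick, with at least two cached, it tests whether the first two's X separation exceeds MaxDistanceBeforeGrowing.
; The branch does nothing yet; the excess-distance calculation and Owner reference are left unconnected, so no camera is changed.
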(event `self.ReceiveBeginPlay`
  ;[1 1 1] Begin Play
  (`parent.ReceiveBeginPlay`)
  (`KismetSystemLibrary.Delay` 1.0)
  (bind _outactors (`GameplayStatics.GetAllActorsOfClass` "/Script/DiamondProject.DiamondProjectCharacter"))
  (set `self.playersInstance` _outactors))

(event `self.ReceiveTick`
  (params (DeltaSeconds :type "Float (single-precision)"))
  (bind _playersinstance (`self.playersInstance`))
  (bind _returnvalue_x (`KismetMathLibrary.BreakVector` (`Actor.K2_GetActorLocation` (`|GetArrayItem` _playersinstance))))
  (bind _returnvalue_x_2 (`KismetMathLibrary.BreakVector` (`Actor.K2_GetActorLocation` (`|GetArrayItem` _playersinstance 1))))
  ;[1 1 1] Tick
  (`parent.ReceiveTick` DeltaSeconds)
  (if (>= (`KismetArrayLibrary.Array_Length` (`self.playersInstance`)) 2)
    (if (< (`self.maxDistanceBeforeGrowing`) (`KismetMathLibrary.Abs` (- _returnvalue_x _returnvalue_x_2)))
      _)))