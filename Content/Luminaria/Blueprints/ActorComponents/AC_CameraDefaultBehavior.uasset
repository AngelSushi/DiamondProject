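; AC_CameraDefaultBehavior is an actor component that keeps its owner, presumably a camera, centred between the player characters.
; After a one-second delay on BeginPlay, it caches every DiamondProjectCharacter once.
; Each tick, with at least two characters cached, it moves the owner to their average X and Z, raised by a fixed height, while preserving its Y, suggesting a side-view camera.
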(event `self.ReceiveBeginPlay`
  (`parent.ReceiveBeginPlay`)
  (`KismetSystemLibrary.Delay` 1.0)
  (bind _outactors (`GameplayStatics.GetAllActorsOfClass` "/Script/DiamondProject.DiamondProjectCharacter"))
  (set `self.playersInstance` _outactors))

(event `self.ReceiveTick`
  (params (DeltaSeconds :type "Float (single-precision)"))
  (bind _playersinstance (`self.playersInstance`))
  (bind (_returnvalue_x _returnvalue_y) (`KismetMathLibrary.BreakVector` (`Actor.K2_GetActorLocation` (`self.owner`))))
  (if (>= (`KismetArrayLibrary.Array_Length` (`self.playersInstance`)) 2)
    (set `self.newCamLocation` (0.0 0.0 0.0))
    (for _array_element _playersinstance
      (bind (_returnvalue_x_2 _returnvalue_y_2 _returnvalue_z) (`KismetMathLibrary.BreakVector` (`Actor.K2_GetActorLocation` _array_element)))
      (set `self.newCamLocation` (+ (`self.newCamLocation`) (`KismetMathLibrary.MakeVector` _returnvalue_x_2 _returnvalue_y (+ _returnvalue_z 45.0)))))
    (`Actor.K2_SetActorLocation` (`self.owner`) (/ (`self.newCamLocation`) (`KismetArrayLibrary.Array_Length` _playersinstance)) false false)))