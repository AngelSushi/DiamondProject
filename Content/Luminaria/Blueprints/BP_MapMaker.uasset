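; BP_MapMaker is an actor that builds map visuals for the level's camera areas through its CreateMap function.
; CreateMap finds every BP_CameraArea and derives its Y/Z bounds from actor location and box extent.
; It scales each area's MapPlane to that size, dividing by 100 and swapping axes so height drives plane X, then applies M_Room.
; The event graph and construction script are empty, so nothing here calls CreateMap.
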(fn `CreateMap`
  (bind _outactors (`GameplayStatics.GetAllActorsOfClass` "/Game/Luminaria/Blueprints/BP_CameraArea.BP_CameraArea_C"))
  (for _array_element _outactors
    (bind _mapplane (`CameraArea.MapPlane` _array_element))
    (bind _returnvalue (`self.K2_GetActorLocation` _array_element))
    (bind _boxextent (`BoxComponent.BoxExtent` (`CameraArea.BoxCollision` _array_element)))
    (bind (_x _y) (`KismetMathLibrary.BreakVector2D` (`KismetMathLibrary.MakeVector2D` (+ (.y _returnvalue) (.y _boxextent)) (+ (.z _returnvalue) (.z _boxextent)))))
    (bind (_x_2 _y_2) (`KismetMathLibrary.BreakVector2D` (`KismetMathLibrary.MakeVector2D` (- (.y _returnvalue) (.y _boxextent)) (- (.z _returnvalue) (.z _boxextent)))))
    (`SceneComponent.SetWorldScale3D` _mapplane (/ (`KismetMathLibrary.MakeVector` (- _y _y_2) (- _x _x_2) 1.0) (100.0 100.0 1.0)))
    (`PrimitiveComponent.SetMaterial` _mapplane 0 "/Game/Luminaria/Materials/M_Room.M_Room")))

(fn `UserConstructionScript`)