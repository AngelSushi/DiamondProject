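; Pushable box that a player character can push or pull while in its Forward trigger, provided the controller's LightValue is high enough.
; Overlap and button state gate CanPush and flip permission, while Tick slows the character and interpolates the box along world Y by stick direction.
; A downward trace flags Destroy past a height gap, but the destroy logic is unwired and no respawn is implemented.
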(event `self.ReceiveBeginPlay`
  (set `self.defaultPosition` (`self.K2_GetActorLocation`)))

(event `self.ReceiveTick`
  (params (DeltaSeconds :type "Float (single-precision)"))
  (bind (_returnvalue_x _returnvalue_y _returnvalue_z) (`KismetMathLibrary.BreakVector` (`self.K2_GetActorLocation`)))
  (bind (_returnvalue_x_2 _returnvalue_y_2) (`KismetMathLibrary.BreakVector` (`self.GetActorScale3D`)))
  (bind _as_bp_top_down_character (`self.As BP Top Down Character`))
  (bind _cubespeed (`self.cubeSpeed`))
  (bind _move_value (`/Game/TopDown/Blueprints/BP_TopDownCharacter.Move value` (`self.As BP Top Down Character`)))
  (bind _charactermovement (`Character.CharacterMovement` _as_bp_top_down_character))
  (bind _returnvalue (- (`self.K2_GetActorLocation`) (+ (`KismetMathLibrary.Vector_Left`) (`KismetMathLibrary.MakeVector` 0.0 (/ (* _returnvalue_y_2 100.0) 2.0)))))
  (`|ExecutionSequence`
    (:`then_0`
      ;[1 1 1] Manage Pushing/Pulling By Player
      (if (`KismetSystemLibrary.IsValid` _as_bp_top_down_character)
        (if (`/Game/TopDown/Blueprints/BP_TopDownCharacter.buttonPushPressed` _as_bp_top_down_character)
          (if (`self.isInZone`)
            (if (>= (`/Game/Luminaria/Config/PC_Player.LightValue` (stale `self.forward.OnComponentBeginOverlap` _aspc_player)) (`self.lightValueNeeded`))
              (set `CharacterMovementComponent.MaxWalkSpeed` 60.0 _charactermovement)
              (if (`/Game/TopDown/Blueprints/BP_TopDownCharacter.canPush` _as_bp_top_down_character)
                (if (== _move_value (0.0 0.0))
                  _
                  (elif (> (`KismetMathLibrary.BreakVector2D` _move_value) 0.0)
                    (set `self.isPushing` true)
                    (set `self.isPulling` false)
                    (`self.Speed/direction` true _cubespeed)
                    (else
                      (set `self.isPulling` true)
                      (set `self.isPushing` false)
                      (`self.Speed/direction` true (* _cubespeed -1.0))))))
              (else
                (`self.StopPushing` null :!label _label)
                (set `CharacterMovementComponent.MaxWalkSpeed` 600.0 _charactermovement :!label _label_2)))
            (else
              (goto _label)))
          (else
            (goto _label_2)))))
    (:`then_1`
      (bind _returnvalue_2 (`PlayerManager.GetAllCharactersRef` (subsystem `PlayerManager`)))
      (bind _outhits (`KismetSystemLibrary.LineTraceMulti` _returnvalue (+ _returnvalue (* (`KismetMathLibrary.Vector_Down`) 10000.0)) "TraceTypeQuery3" false (`|MakeArray` (`|GetArrayItem` _returnvalue_2) (`|GetArrayItem` _returnvalue_2 1) null :!type "Actor Object Reference") "ForDuration"))
      (if (> (`KismetArrayLibrary.Array_Length` _outhits) 0)
        (bind (_returnvalue_x_3 _returnvalue_y_3 _returnvalue_z_2) (`KismetMathLibrary.BreakVector` (`self.K2_GetActorLocation` (`.HitActor` (`GameplayStatics.BreakHitResult` (`|GetArrayItem` _outhits))))))
        (if (and (not (`self.destroy`)) (>= (`KismetMathLibrary.Abs` (- _returnvalue_z _returnvalue_z_2)) (`self.destroyDistance`)))
          (set `self.destroy` true))))))

(event `self.forward.OnComponentBeginOverlap`
  (params (OverlappedComponent :type "PrimitiveComponent Object Reference") (OtherActor :type "Actor Object Reference") (OtherComp :type "PrimitiveComponent Object Reference") (OtherBodyIndex :type Integer) (bFromSweep :type Boolean) (SweepResult :type "HitResult Structure (by ref)"))
  (bind _asbp_top_down_character (cast `/Game/TopDown/Blueprints/BP_TopDownCharacter` OtherActor))
  (set `self.As BP Top Down Character` _asbp_top_down_character)
  (bind _aspc_player (cast `/Game/Luminaria/Config/PC_Player` (`Pawn.GetController` _asbp_top_down_character)))
  (bind _output_get (set `self.isInZone` true))
  (`KismetSystemLibrary.PrintString` (`KismetStringLibrary.Conv_BoolToString` _output_get))
  (if (>= (`/Game/Luminaria/Config/PC_Player.LightValue` _aspc_player) (`self.lightValueNeeded`))
    (set `self.goodLightVallue` true)
    (`self.startPushing` _asbp_top_down_character)
    (else
      (set `self.goodLightVallue` false)
      (`self.StopPushing` _asbp_top_down_character))))

(event `self.forward.OnComponentEndOverlap`
  (params (OverlappedComponent :type "PrimitiveComponent Object Reference") (OtherActor :type "Actor Object Reference") (OtherComp :type "PrimitiveComponent Object Reference") (OtherBodyIndex :type Integer))
  (bind _asbp_top_down_character (cast `/Game/TopDown/Blueprints/BP_TopDownCharacter` OtherActor))
  (bind _output_get (set `self.As BP Top Down Character` _asbp_top_down_character))
  (set `self.isInZone` false)
  (if (not (>= (`/Game/Luminaria/Config/PC_Player.LightValue` (stale `self.forward.OnComponentBeginOverlap` _aspc_player)) (`self.lightValueNeeded`)))
    (`self.StopPushing` _output_get)))

(event `startPushing`
  (params (Character :type "/Game/TopDown/Blueprints/BP_TopDownCharacter Object Reference"))
  (`/Engine/EditorBlueprintResources/StandardMacros.IsValid` Character
    (:`Is Valid`
      (`KismetSystemLibrary.PrintString` "Start My Pus")
      (set `/Game/TopDown/Blueprints/BP_TopDownCharacter.canPush` true Character)
      (if (`/Game/TopDown/Blueprints/BP_TopDownCharacter.buttonPushPressed` Character)
        (bind _asdiamond_project_player_controller (cast `DiamondProjectPlayerController` (`Pawn.GetController` (stale `StopPushing` Character))))
        (set `DiamondProjectPlayerController.bCanFlip` false _asdiamond_project_player_controller)))))

(event `self.Cube.OnComponentBeginOverlap`
  (params (OverlappedComponent :type "PrimitiveComponent Object Reference") (OtherActor :type "Actor Object Reference") (OtherComp :type "PrimitiveComponent Object Reference") (OtherBodyIndex :type Integer) (bFromSweep :type Boolean) (SweepResult :type "HitResult Structure (by ref)"))
  ;[1 1 1] Destroy And Respawn
)

(event `StopPushing`
  (params (Character :type "/Game/TopDown/Blueprints/BP_TopDownCharacter Object Reference"))
  (`/Engine/EditorBlueprintResources/StandardMacros.IsValid` Character
    (:`Is Valid`
      (set `/Game/TopDown/Blueprints/BP_TopDownCharacter.canPush` false Character)
      (bind _asdiamond_project_player_controller (cast `DiamondProjectPlayerController` (`Pawn.GetController` Character)))
      (set `DiamondProjectPlayerController.bCanFlip` true _asdiamond_project_player_controller))))

(fn `UserConstructionScript`)