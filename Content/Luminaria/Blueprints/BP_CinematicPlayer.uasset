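; Trigger box that plays an assigned level sequence once, when its begin-overlap count reaches two, presumably both players.
; It stores and removes top-level widgets, then plays the sequence with the HUD hidden.
; It disables Pc_PlayerElectric movement, using a Delay inside the character loop timed to the sequence length to re-enable it.
; FinalCinematicFunc, not called here, hides all characters when the sequence is LS_EndRoom.
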(event `self.Box.OnComponentBeginOverlap`
  (params (OverlappedComponent :type "PrimitiveComponent Object Reference") (OtherActor :type "Actor Object Reference") (OtherComp :type "PrimitiveComponent Object Reference") (OtherBodyIndex :type Integer) (bFromSweep :type Boolean) (SweepResult :type "HitResult Structure (by ref)"))
  (bind _result (`/Engine/EditorBlueprintResources/StandardMacros.IncrementInt` (`self.PlayerIn`))
    (:`  `
      (if (== _result 2)
        (`KismetSystemLibrary.PrintString` "Enter Box")
        (`/Engine/EditorBlueprintResources/StandardMacros.DoOnce` false
          (:`Completed`
            (bind _foundwidgets (`WidgetBlueprintLibrary.GetAllWidgetsOfClass` "/Script/UMG.UserWidget"))
            (for _array_element _foundwidgets
              (`KismetArrayLibrary.Array_Add` (`self.AllWidgets`) _array_element)
              (`Widget.RemoveFromParent` _array_element))
            (bind (_outactor _returnvalue) (`LevelSequencePlayer.CreateLevelSequencePlayer` (`self.SequenceToPlay`) (make `MovieSceneSequencePlaybackSettings` false (struct) 1.0 0.0 false false false false false true)))
            (`MovieSceneSequencePlayer.Play` (`LevelSequenceActor.SequencePlayer` _outactor))
            (`MovieSceneSequencePlayer.Play` _returnvalue)
            (for _array_element_2 (`PlayerManager.GetAllCharactersRef` (subsystem `PlayerManager`))
              (bind _aspc_player_electric (cast `/Game/Luminaria/Config/Pc_PlayerElectric` (`DiamondProjectCharacter.GetLuminariaController` _array_element_2)))
              (set `DiamondProjectPlayerController.bCanMove` false _aspc_player_electric)
              (bind (_returnvalue_frame _returnvalue_framerate) (break `QualifiedFrameTime` (`MovieSceneSequencePlayer.GetEndTime` _returnvalue)))
              (`KismetSystemLibrary.Delay` (`KismetMathLibrary.Conv_IntToDouble` (/ (`.Value` (break `FrameNumber` _returnvalue_frame)) (`KismetMathLibrary.BreakFrameRate` _returnvalue_framerate))))
              (set `DiamondProjectPlayerController.bCanMove` true _aspc_player_electric))))))))

(fn `FinalCinematicFunc`
  (if (== (`self.SequenceToPlay`) "/Game/Cinematic/LS_EndRoom.LS_EndRoom")
    (for _array_element (`PlayerManager.GetAllCharactersRef` (subsystem `PlayerManager`))
      (`self.SetActorHiddenInGame` _array_element true))))

(fn `UserConstructionScript`)