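; BP_FInalCristal is a crystal actor whose material can be animated to glow.
; BeginPlay creates a dynamic instance of the crystal material on its mesh, zeroing the Value parameter and setting SecondColor to white.
; StartGlowing plays the Glowing timeline, which feeds its track into Value on each update.
; ActivateCrystal only resets Value to zero, followed by a constant comparison that leads nowhere.
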(event `self.ReceiveBeginPlay`
  (bind _returnvalue (`PrimitiveComponent.CreateDynamicMaterialInstance` (`self.MeshComponent`) 0 "/Game/Luminaria/Materials/M_Plateform_Crystal_002.M_Plateform_Crystal_002" "None"))
  (set `self.OrbMaterial` _returnvalue)
  (`MaterialInstanceDynamic.SetScalarParameterValue` _returnvalue "Value" 0.0)
  (`MaterialInstanceDynamic.SetVectorParameterValue` _returnvalue "SecondColor" (struct :`R` 1.0 :`G` 1.0 :`B` 1.0 :`A` 1.0)))

(event `StartGlowing`
  (bind (_direction _time) (`Timeline|Glowing`)
    (:`Update`
      (`MaterialInstanceDynamic.SetScalarParameterValue` (`self.OrbMaterial`) "Value" _time))))

(fn `ActivateCrystal`
  (`MaterialInstanceDynamic.SetScalarParameterValue` (`self.OrbMaterial`) "Value" 0.0)
  (if (`KismetMathLibrary.NearlyEqual_FloatFloat` 0.0 1.0 0.02)
    _))

(fn `UserConstructionScript`)