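; BP_DialogSpawner displays a French dialog line as world-space text with a typewriter reveal.
; OnDisplayDialog searches the Dialogues data table for the row matching its dialog ID and creates a blue-green emissive material instance for the text.
; Tick reveals characters on a timer and repositions the text from the player's X and main camera's location, offset upward.
; Tick also clears the text after a delay given by GetTextDuration.
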(event `self.OnDisplayDialog`
  (bind _targetcolor (`self.TargetColor`))
  (bind (_r _g _b) (`KismetMathLibrary.BreakColor` _targetcolor))
  (set `self.IsDisplayed` true)
  (bind _outrownames (`DataTableFunctionLibrary.GetDataTableRowNames` "/Game/Luminaria/Dialogs/Dialogues_-_Feuille_1__1_.Dialogues_-_Feuille_1__1_"))
  (for _array_element _outrownames
    (bind _returnvalue (`|GetDataTableRow` "/Game/Luminaria/Dialogs/Dialogues_-_Feuille_1__1_.Dialogues_-_Feuille_1__1_" _array_element)
      (:`then`
        (if (== (`self.GetDialogID`) (break `/Game/Luminaria/Dialogs/DialogStruct` _returnvalue))
          (set `self.DialogText` (`KismetTextLibrary.Conv_StringToText` (`.FR_fr_7_F936D5A743502F64E334B28CB2830EC5` (break `/Game/Luminaria/Dialogs/DialogStruct` _returnvalue))))
          (bind _returnvalue_2 (`PrimitiveComponent.CreateDynamicMaterialInstance` (`self.Border`) 0 "/Game/Luminaria/Materials/M_BlueGreenEmissive.M_BlueGreenEmissive" "None"))
          (set `self.BorderMaterial` _returnvalue_2)
          (bind _returnvalue_3 (`MaterialInstanceDynamic.K2_GetVectorParameterValue` _returnvalue_2 "Color"))
          (set `self.TargetColor` _returnvalue_3)
          (set `self.OriginColor` (`KismetMathLibrary.MakeColor` _r _g _b))
          (`MaterialInstanceDynamic.SetVectorParameterValue` _returnvalue_2 "Color" _targetcolor)
          (set `self.isLiving` false)
          (break))))))

(event `self.ReceiveTick`
  (params (DeltaSeconds :type "Float (single-precision)"))
  (`|ExecutionSequence`
    (:`then_0`
      (`self.TransitionAppearance` DeltaSeconds))
    (:`then_1`
      (`self.ManagePosition`))
    (:`then_2`
      (if (not (`self.isLiving`))
        (set `self.isLiving` true)
        (`KismetSystemLibrary.Delay` (`self.GetTextDuration`))
        (`TextRenderComponent.K2_SetText` (`self.Border`) (`KismetTextLibrary.Conv_StringToText` ""))
        (set `self.IsDisplayed` false)))))

(fn `ManagePosition`
  (bind _returnvalue (`PlayerManager.GetOnePlayer` (subsystem `PlayerManager`)))
  (bind (_returnvalue_x _returnvalue_y) (`KismetMathLibrary.BreakVector` (/ (`TextRenderComponent.GetTextLocalSize` (`self.Border`)) 2)))
  (`/Engine/EditorBlueprintResources/StandardMacros.IsValid` _returnvalue
    (:`Is Valid`
      (bind _returnvalue_2 (`DiamondProjectCharacter.GetMainCamera` _returnvalue))
      (`/Engine/EditorBlueprintResources/StandardMacros.IsValid` _returnvalue_2
        (:`Is Valid`
          (`SceneComponent.K2_SetWorldLocation` (`self.Border`) (`KismetMathLibrary.MakeVector` (.x (`self.K2_GetActorLocation` _returnvalue)) (- (.y (`self.K2_GetActorLocation` _returnvalue_2)) _returnvalue_y) (+ (.z (`self.K2_GetActorLocation` _returnvalue_2)) 500.0)) false false))))))

(fn `TransitionAppearance`
  (params (DeltaTime :type "Float (double-precision)"))
  (if (`self.IsDisplayed`)
    (bind _output_get (set `self.Timer` (+ (`self.Timer`) DeltaTime)))
    (if (>= _output_get (`self.MaxTimerAppearance`))
      (set `self.Timer` 0.0)
      (bind _result (`/Engine/EditorBlueprintResources/StandardMacros.IncrementInt` (`self.CharacterIndex`))
        (:`  `
          (`TextRenderComponent.K2_SetText` (`self.Border`) (`KismetTextLibrary.Conv_StringToText` (`KismetStringLibrary.GetSubstring` (`KismetTextLibrary.Conv_TextToString` (`self.DialogText`)) 0 _result))))))))

(fn `UserConstructionScript`)