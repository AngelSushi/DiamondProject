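; BP_GrowthOrb is a pulsing pickup orb that unlocks growing for all player characters when a DiamondProjectCharacter touches it.
; Tick advances a timer by GrowthSpeed and ping-pongs the Alpha parameter of a dynamic M_Orb material between minimum and maximum intensity.
; On mesh overlap, it calls SetCanGrow on every character from the PlayerManager and destroys itself within that loop.
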(event `self.ReceiveBeginPlay`
  (bind _returnvalue (`PrimitiveComponent.CreateDynamicMaterialInstance` (`self.MeshComponent`) 0 "/Game/Luminaria/Materials/M_Orb.M_Orb" "None"))
  (set `self.OrbMaterial` _returnvalue)
  (`MaterialInstanceDynamic.SetScalarParameterValue` _returnvalue "Alpha" (`self.MinIntensity`)))

(event `self.ReceiveTick`
  (params (DeltaSeconds :type "Float (single-precision)"))
  (bind _output_get (set `self.Timer` (+ (* DeltaSeconds (`self.GrowthSpeed`)) (`self.Timer`))))
  (bind _output_get_2 (set `self.TargetIntensity` (`MathUtilities.PingPongFloat` _output_get (`self.MinIntensity`) (`self.MaxIntensity`))))
  (`MaterialInstanceDynamic.SetScalarParameterValue` (`self.OrbMaterial`) "Alpha" _output_get_2))

(event `self.MeshComponent.OnComponentBeginOverlap`
  (params (OverlappedComponent :type "PrimitiveComponent Object Reference") (OtherActor :type "Actor Object Reference") (OtherComp :type "PrimitiveComponent Object Reference") (OtherBodyIndex :type Integer) (bFromSweep :type Boolean) (SweepResult :type "HitResult Structure (by ref)"))
  (cast `DiamondProjectCharacter` OtherActor)
  (for _array_element (`PlayerManager.GetAllCharactersRef` (subsystem `PlayerManager`))
    (`DiamondProjectCharacter.SetCanGrow` _array_element true)
    (`self.K2_DestroyActor`)))

(fn `UserConstructionScript`)