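; Link Blueprint that colors a dissolve-material mesh to reflect the state of the two players.
; Creates a dynamic material on BeginPlay and records the players' Y-axis order once both register with PlayerManager.
; Each tick sets both player colors, a distance alpha and a blend value from the first player's clamped LightEnergy, inverted when the current order differs from the recorded one.
; DispatchColors is an empty stub.
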(event `self.ReceiveBeginPlay`
  (bind _returnvalue (`PrimitiveComponent.CreateDynamicMaterialInstance` (`self._mesh`) 0 "/Game/ParticlesFX/Materials/M_Dissolve_Link.M_Dissolve_Link" "None"))
  (set `self.LinkMaterial` _returnvalue)
  (add `PlayerManager.OnPlayerRegister` (subsystem `PlayerManager`) (delegate `OnPlayerRegisterEvent`)))

(event `OnPlayerRegisterEvent`
  (params (Character :type "DiamondProjectCharacter Object Reference"))
  (`self.DispatchColors` Character)
  (if (== (`KismetArrayLibrary.Array_Length` (`PlayerManager.GetAllCharactersRef` (subsystem `PlayerManager`))) 2)
    (`self.GetOrderedPlayers` (`self.OrderedPlayers`))))

(event `self.ReceiveTick`
  (params (DeltaSeconds :type "Float (single-precision)"))
  (bind _returnvalue (`self.GetDistanceAlpha`))
  (bind _returnvalue_2 (subsystem `PlayerManager`))
  (bind _linkmaterial (`self.LinkMaterial`))
  (bind _updateorderedplayers (`self.UpdateOrderedPlayers`))
  (bind _linkmaterial_2 (`self.LinkMaterial`))
  (bind _returnvalue_3 (`PlayerManager.GetOrderedPlayers` _returnvalue_2))
  (bind _returnvalue_4 (`PlayerManager.GetAllCharactersRef` _returnvalue_2))
  (bind _returnvalue_5 (`PlayerManager.GetAllCharactersRef` (subsystem `PlayerManager`)))
  (bind _output (`|GetArrayItem` _returnvalue_5))
  (bind _returnvalue_6 (`DiamondProjectCharacter.GetPlayerColor` (`|GetArrayItem` _returnvalue_4 (`|GetArrayItem` _returnvalue_3 1))))
  (bind _returnvalue_7 (`DiamondProjectCharacter.GetPlayerColor` (`|GetArrayItem` _returnvalue_4 (`|GetArrayItem` _returnvalue_3))))
  (bind _returnvalue_8 (`KismetMathLibrary.FClamp` (/ (`DiamondProjectCharacter.LightEnergy` _output) 100000.0)))
  (`KismetArrayLibrary.Array_Clear` _updateorderedplayers)
  (`self.GetOrderedPlayers` _updateorderedplayers)
  (if (!= (`KismetArrayLibrary.Array_Length` (`self.OrderedPlayers`)) 0)
    (if (and (`KismetSystemLibrary.IsValid` _output) (`KismetSystemLibrary.IsValid` (`|GetArrayItem` _returnvalue_5 1)))
      (if (!= (`|GetArrayItem` (`self.UpdateOrderedPlayers`)) (`|GetArrayItem` (`self.OrderedPlayers`)))
        (`MaterialInstanceDynamic.SetVectorParameterValue` _linkmaterial_2 "FirstColor" (`KismetMathLibrary.Conv_ColorToLinearColor` _returnvalue_6))
        (`MaterialInstanceDynamic.SetVectorParameterValue` _linkmaterial_2 "SecondColor" (`KismetMathLibrary.Conv_ColorToLinearColor` _returnvalue_7))
        (`MaterialInstanceDynamic.SetScalarParameterValue` _linkmaterial "Value" (- 1.0 _returnvalue_8))
        (`MaterialInstanceDynamic.SetScalarParameterValue` _linkmaterial "DistanceAlpha" _returnvalue)
        (else
          (`MaterialInstanceDynamic.SetVectorParameterValue` _linkmaterial_2 "FirstColor" (`KismetMathLibrary.Conv_ColorToLinearColor` _returnvalue_6))
          (`MaterialInstanceDynamic.SetVectorParameterValue` _linkmaterial_2 "SecondColor" (`KismetMathLibrary.Conv_ColorToLinearColor` _returnvalue_7))
          (`MaterialInstanceDynamic.SetScalarParameterValue` _linkmaterial "Value" _returnvalue_8)
          (`MaterialInstanceDynamic.SetScalarParameterValue` _linkmaterial "DistanceAlpha" _returnvalue))))))

(fn `DispatchColors`
  (params (Player :type "DiamondProjectCharacter Object Reference"))
  (bind _returnvalue (`KismetArrayLibrary.Array_Length` (`PlayerManager.GetAllCharactersRef` (subsystem `PlayerManager`))))
  (`|ExecutionSequence`
    (:`then_0`
      (if (== _returnvalue 1)
        _))
    (:`then_1`
      (if (== _returnvalue 2)
        _))))

(fn `GetOrderedPlayers`
  (params (OrderedPlayersList :type "Array of DiamondProjectCharacter Object Reference"))
  (locals (MinsY :type "Array of Float (double-precision)"))
  (bind _indexofminvalue (`KismetMathLibrary.MinOfFloatArray` (`local.MinsY`)))
  (bind _returnvalue (`PlayerManager.GetAllCharactersRef` (subsystem `PlayerManager`)))
  (for _array_element _returnvalue
    (bind (_returnvalue_x _returnvalue_y) (`KismetMathLibrary.BreakVector` (`self.K2_GetActorLocation` _array_element)))
    (`KismetArrayLibrary.Array_Add` (`local.MinsY`) _returnvalue_y))
  (`KismetArrayLibrary.Array_Add` OrderedPlayersList (`|GetArrayItem` _returnvalue _indexofminvalue))
  (`KismetArrayLibrary.Array_Add` OrderedPlayersList (`|GetArrayItem` _returnvalue (`KismetMathLibrary.Wrap` (+ _indexofminvalue 1) 0 1))))

(fn `UserConstructionScript`)