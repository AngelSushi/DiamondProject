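; Camera area Blueprint for area 28 that drives a scripted camera move when the player manager reports a change to area ID 1000.
; It subscribes to the manager's area-change event at BeginPlay, then switches the player's main camera to a GoTo behavior.
; The target keeps the camera's current X and takes Y and Z from the GoTo component.
; The behavior is set to hand over to Dynamic with a delay on arrival.
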(event `self.ReceiveBeginPlay`
  (`KismetSystemLibrary.PrintString` "Start 028 Area")
  (add `PlayerManager.OnChangeNewArea` (subsystem `PlayerManager`) (delegate `OnChangeNewArea`)))

(event `OnChangeNewArea`
  (params (AreaID :type Integer))
  (bind (_returnvalue_x _returnvalue_y _returnvalue_z) (`KismetMathLibrary.BreakVector` (`SceneComponent.K2_GetComponentLocation` (`self.GoTo`))))
  (if (== AreaID 1000)
    (bind _returnvalue (`DiamondProjectCharacter.GetMainCamera` (`PlayerManager.GetOnePlayer` (subsystem `PlayerManager`))))
    (bind _returnvalue_2 (`LuminariaCamera.SwitchBehaviorFromBlueprint` _returnvalue "GOTO"))
    (bind _asgo_to_behavior (cast `GoToBehavior` _returnvalue_2))
    (bind _returnvalue_x_2 (`KismetMathLibrary.BreakVector` (`self.K2_GetActorLocation` _returnvalue)))
    (set `GoToBehavior.GoTo` (`KismetMathLibrary.MakeVector` _returnvalue_x_2 _returnvalue_y _returnvalue_z) _asgo_to_behavior)
    (set `GoToBehavior.NextBehavior` "DYNAMIC" _asgo_to_behavior)
    (set `GoToBehavior.DelayAtReach` 3.0 _asgo_to_behavior)))

(fn `UserConstructionScript`)