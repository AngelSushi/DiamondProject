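; BP_Camera is a camera Blueprint that switches between Default, Leader and Dynamic behaviors, each implemented as a separate component.
; On BeginPlay it adds the component matching CameraBehavior and records that value as LastBehavior.
; Tick compares the two values and, when they differ, destroys the old component and adds the new one.
; LastBehavior is never updated in Tick, so the swap repeats every frame after a change.
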(event `self.ReceiveBeginPlay`
  (bind _camerabehavior (`self.CameraBehavior`))
  (set `self.LastBehavior` _camerabehavior)
  (switch `ECameraBehavior` _camerabehavior
    (:`DEFAULT`
      (bind _returnvalue (`AddComponent|NODE_AddBP_DefaultBehaviorComponent-0`))
      (set `self.DefaultBehaviorComponent` _returnvalue))
    (:`LEADER`
      (bind _returnvalue_2 (`AddComponent|NODE_AddBP_LeaderBehaviorComponent-0`))
      (set `self.LeaderBehaviorComponent` _returnvalue_2))
    (:`DYNAMIC`
      (bind _returnvalue_3 (`AddComponent|NODE_AddBP_CameraDynamicComponent-0`))
      (set `self.DynamicBehaviorComponent` _returnvalue_3))))

(event `self.ReceiveTick`
  (params (DeltaSeconds :type "Float (single-precision)"))
  (bind _defaultbehaviorcomponent (`self.DefaultBehaviorComponent`))
  (bind _leaderbehaviorcomponent (`self.LeaderBehaviorComponent`))
  (bind _dynamicbehaviorcomponent (`self.DynamicBehaviorComponent`))
  (if (!= (`KismetMathLibrary.Conv_ByteToDouble` (`self.LastBehavior`)) (`KismetMathLibrary.Conv_ByteToDouble` (`self.CameraBehavior`)))
    (`|ExecutionSequence`
      (:`then_0`
        (switch `ECameraBehavior` (`self.LastBehavior`)
          (:`DEFAULT`
            (`/Engine/EditorBlueprintResources/StandardMacros.IsValid` _defaultbehaviorcomponent
              (:`Is Valid`
                (`ActorComponent.K2_DestroyComponent` _defaultbehaviorcomponent))))
          (:`LEADER`
            (`/Engine/EditorBlueprintResources/StandardMacros.IsValid` _leaderbehaviorcomponent
              (:`Is Valid`
                (`ActorComponent.K2_DestroyComponent` _leaderbehaviorcomponent))))
          (:`DYNAMIC`
            (`/Engine/EditorBlueprintResources/StandardMacros.IsValid` _dynamicbehaviorcomponent
              (:`Is Valid`
                (`ActorComponent.K2_DestroyComponent` _dynamicbehaviorcomponent))))))
      (:`then_1`
        (switch `ECameraBehavior` (`self.CameraBehavior`)
          (:`DEFAULT`
            (bind _returnvalue (`AddComponent|NODE_AddBP_DefaultBehaviorComponent-1`))
            (set `self.DefaultBehaviorComponent` _returnvalue))
          (:`LEADER`
            (bind _returnvalue_2 (`AddComponent|NODE_AddBP_LeaderBehaviorComponent-1`))
            (set `self.LeaderBehaviorComponent` _returnvalue_2))
          (:`DYNAMIC`
            (bind _returnvalue_3 (`AddComponent|NODE_AddBP_CameraDynamicComponent-1`))
            (set `self.DynamicBehaviorComponent` _returnvalue_3)))))))

(fn `UserConstructionScript`)