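; Player controller for the electric character in Luminaria, handling interact input and light energy transfer between players.
; The transfer input, gated by a minimum LightValue, calls SendOrb, which resolves sender and receiver through the player manager and spawns a BP_ElectricOrb.
; SendOrb then debits the sender through LightTransfer, which also has a receiver branch.
; LightTransfer only changes and pushes LightValue to the character below a cap and when the camera's current area allows growth.
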(event `Init`
  ;[1 0 0.3592] Get All Ref to not do it later
  (cast `/Game/TopDown/Blueprints/BP_TopDownCharacter` (`self.K2_GetPawn`)))

(event `EnhancedInput|/Game/Luminaria/Inputs/IA_LightTransfert`
  (params (ActionValue :type Boolean) (ElapsedSeconds :type "Float (double-precision)") (TriggeredSeconds :type "Float (double-precision)") (InputAction :type "InputAction Object Reference" :default "/Game/Luminaria/Inputs/IA_LightTransfert.IA_LightTransfert"))
  (:`Triggered`
    (if (> (`self.LightValue`) 10.0)
      (`self.SendOrb`)
      (`self.OnLightTransfered`))))

(event `EnhancedInput|/Game/Luminaria/Inputs/IA_Interact`
  (params (ActionValue :type Boolean) (ElapsedSeconds :type "Float (double-precision)") (TriggeredSeconds :type "Float (double-precision)") (InputAction :type "InputAction Object Reference" :default "/Game/Luminaria/Inputs/IA_Interact.IA_Interact"))
  (:`Triggered`
    (set `self.isInteracting` true))
  (:`Completed`
    (set `self.isInteracting` false)))

(fn `Light Transfer`
  (params (IsSender :type Boolean))
  (bind _returnvalue (`self.GetPlayer`))
  (bind _lightvalue (`self.LightValue`))
  (bind _lightvalue_2 (`self.LightValue`))
  (bind _returnvalue_2 (`DiamondProjectCharacter.GetMainCamera` (`self.GetPlayer`)))
  (bind _returnvalue_3 (`LuminariaCamera.GetCurrentArea` _returnvalue_2))
  (bind _returnvalue_4 (`CameraArea.CanGrow` _returnvalue_3))
  (if _returnvalue_4
    (if IsSender
      (if (< _lightvalue 90.0)
        (bind _output_get (set `self.LightValue` (- _lightvalue (`self.TransferValue`))))
        (bind _asbp_top_down_character (cast `/Game/TopDown/Blueprints/BP_TopDownCharacter` _returnvalue))
        (`/Game/TopDown/Blueprints/BP_TopDownCharacter.SetLightEnergyEvent` _asbp_top_down_character _output_get))
      (elif (< _lightvalue_2 90.0)
        (bind _output_get_2 (set `self.LightValue` (+ _lightvalue_2 (`self.TransferValue`))))
        (bind _asbp_top_down_character_2 (cast `/Game/TopDown/Blueprints/BP_TopDownCharacter` _returnvalue))
        (`/Game/TopDown/Blueprints/BP_TopDownCharacter.SetLightEnergyEvent` _asbp_top_down_character_2 _output_get_2)))))

(fn `SendOrb`
  (bind _returnvalue (subsystem `PlayerManager`))
  (bind _orbsender (`self.OrbSender`))
  (bind _orbreceiver (`self.OrbReceiver`))
  (bind _returnvalue_2 (`PlayerManager.GetAllControllersRef` (subsystem `PlayerManager`)))
  (for _array_element _returnvalue_2
    (if (== _array_element self)
      (bind _output_get (set `self.OrbSender` _array_element))
      (bind _returnvalue_3 (`PlayerManager.GetOtherPlayer` _returnvalue (`self.GetPlayer` _output_get)))
      (bind _returnvalue_4 (`DiamondProjectCharacter.GetLuminariaController` _returnvalue_3))
      (set `self.OrbReceiver` _returnvalue_4)
      (else
        (bind _output_get_2 (set `self.OrbReceiver` _array_element))
        (bind _returnvalue_5 (`PlayerManager.GetOtherPlayer` _returnvalue (`self.GetPlayer` _output_get_2)))
        (bind _returnvalue_6 (`DiamondProjectCharacter.GetLuminariaController` _returnvalue_5))
        (set `self.OrbSender` _returnvalue_6))))
  (bind _returnvalue_7 (`|SpawnActorFromClass` "/Game/Luminaria/Blueprints/Basics/BP_ElectricOrb.BP_ElectricOrb_C" (`KismetMathLibrary.MakeTransform` (0.0 0.0 0.0) (struct) (0.2 0.2 0.2)) "Undefined" "MultiplyWithRoot" null null))
  (set `ElectricityOrb.orbSender` _orbsender _returnvalue_7)
  (set `ElectricityOrb.orbReceiver` _orbreceiver _returnvalue_7)
  (if (and (`KismetSystemLibrary.IsValid` _orbreceiver) (`KismetSystemLibrary.IsValid` _orbsender))
    (bind _aspc_player_electric (cast `/Game/Luminaria/Config/Pc_PlayerElectric` _orbsender))
    (`self.Light Transfer` _aspc_player_electric true)))

(fn `Update Players State`)

(fn `UserConstructionScript`)