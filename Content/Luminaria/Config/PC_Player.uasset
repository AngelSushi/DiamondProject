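; Player controller for two local players who each hold a light value and can pass some to the other.
; Init caches both top-down pawns and the opposite controller, picked by controller ID.
; Light-transfer input moves a fixed amount if enough light remains, updates both pawns' energy and prints both values.
; Interact input toggles a held flag; UpdatePlayersState is an empty stub with unconnected point-light intensity code.
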(event `Init`
  ;[1 0 0.3592] Get All Ref to not do it later
  (bind _asbp_top_down_character (cast `/Game/TopDown/Blueprints/BP_TopDownCharacter` (`self.K2_GetPawn`)))
  (set `self.RefToPawn` _asbp_top_down_character)
  (if (== (`GameplayStatics.GetPlayerControllerID` self) 0)
    (bind _aspc_player (cast `/Game/Luminaria/Config/PC_Player` (`GameplayStatics.GetPlayerController` 1)))
    (bind _output_get (set `self.RefOtherPlayerController` _aspc_player))
    (bind _asbp_top_down_character_2 (cast `/Game/TopDown/Blueprints/BP_TopDownCharacter` (`self.K2_GetPawn` _output_get)))
    (set `self.RefToOtherPawn` _asbp_top_down_character_2)
    (else
      (bind _aspc_player_2 (cast `/Game/Luminaria/Config/PC_Player` (`GameplayStatics.GetPlayerController` 0)))
      (bind _output_get_2 (set `self.RefOtherPlayerController` _aspc_player_2))
      (bind _asbp_top_down_character_3 (cast `/Game/TopDown/Blueprints/BP_TopDownCharacter` (`self.K2_GetPawn` _output_get_2)))
      (set `self.RefToOtherPawn` _asbp_top_down_character_3))))

(event `EnhancedInput|/Game/Luminaria/Inputs/IA_LightTransfert`
  (params (ActionValue :type Boolean) (ElapsedSeconds :type "Float (double-precision)") (TriggeredSeconds :type "Float (double-precision)") (InputAction :type "InputAction Object Reference" :default "/Game/Luminaria/Inputs/IA_LightTransfert.IA_LightTransfert"))
  (:`Triggered`
    (`self.LightTransfer`)))

(event `EnhancedInput|/Game/Luminaria/Inputs/IA_Interact`
  (params (ActionValue :type Boolean) (ElapsedSeconds :type "Float (double-precision)") (TriggeredSeconds :type "Float (double-precision)") (InputAction :type "InputAction Object Reference" :default "/Game/Luminaria/Inputs/IA_Interact.IA_Interact"))
  (:`Triggered`
    (set `self.isInteracting` true))
  (:`Completed`
    (set `self.isInteracting` false)))

(fn `LightTransfer`
  (bind _transfervalue (`self.TransferValue`))
  (bind _lightvalue (`self.LightValue`))
  (bind _refotherplayercontroller (`self.RefOtherPlayerController`))
  (if (>= _lightvalue 10)
    (bind _output_get (set `self.LightValue` (- _lightvalue _transfervalue)))
    (bind _output_get_2 (set `/Game/Luminaria/Config/PC_Player.LightValue` (+ (`/Game/Luminaria/Config/PC_Player.LightValue` _refotherplayercontroller) _transfervalue) _refotherplayercontroller))
    (`self.Update Players State`)
    (`/Game/TopDown/Blueprints/BP_TopDownCharacter.SetLightEnergy` (`self.RefToPawn`) _output_get)
    (`/Game/TopDown/Blueprints/BP_TopDownCharacter.SetLightEnergy` (`self.RefToOtherPawn`) _output_get_2)
    (`KismetSystemLibrary.PrintString` (`KismetStringLibrary.Concat_StrStr` "Value 1 : " (`KismetStringLibrary.Conv_DoubleToString` _output_get)))
    (`KismetSystemLibrary.PrintString` (`KismetStringLibrary.Concat_StrStr` "Value 2 : " (`KismetStringLibrary.Conv_DoubleToString` _output_get_2)))))

(fn `Update Players State`)

(fn `UserConstructionScript`)