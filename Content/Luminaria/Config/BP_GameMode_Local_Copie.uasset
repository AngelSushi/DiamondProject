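; Local multiplayer game mode that sets up one player per PlayerStart in the level when play begins.
; For each start it creates a local player, adds the IMC_Player Enhanced Input context, then spawns and possesses a BP_TopDownCharacter.
; Index 0 uses the existing first controller; each PC_Player_Copie is collected, then initialized after the loop.
; An unconnected branch that spawns BP_Player instead never runs.
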(event `self.ReceiveBeginPlay`
  (bind _returnvalue (`GameplayStatics.GetPlayerController` 0))
  (bind _returnvalue_2 (`GameplayStatics.GetPlayerController` (`self.Index`)))
  (bind _outactors (`GameplayStatics.GetAllActorsOfClass` "/Script/Engine.PlayerStart"))
  (for (_array_element _array_index) _outactors
    (set `self.Index` _array_index)
    (set `self.Element` _array_element)
    (bind _returnvalue_3 (`GameplayStatics.CreatePlayer` (`self.Index`)))
    (if (> (`self.Index`) 0)
      (message `EnhancedInputSubsystemInterface.AddMappingContext` (pcsubsystem `EnhancedInputLocalPlayerSubsystem` _returnvalue_3) "/Game/Luminaria/Inputs/IMC_Player.IMC_Player" 0 (struct))
      (bind _returnvalue_4 (`|SpawnActorFromClass` "/Game/TopDown/Blueprints/BP_TopDownCharacter.BP_TopDownCharacter_C" (`self.GetTransform` (`self.Element`)) "Undefined" "MultiplyWithRoot" null null))
      (`Controller.Possess` _returnvalue_2 _returnvalue_4)
      (bind _aspc_player_copie (cast `/Game/Luminaria/Config/PC_Player_Copie` _returnvalue_2))
      (`KismetArrayLibrary.Array_Add` (`self.PlayerControllers`) _aspc_player_copie)
      (else
        (message `EnhancedInputSubsystemInterface.AddMappingContext` (pcsubsystem `EnhancedInputLocalPlayerSubsystem` (`GameplayStatics.GetPlayerController` 0)) "/Game/Luminaria/Inputs/IMC_Player.IMC_Player" 0 (struct))
        (bind _returnvalue_5 (`|SpawnActorFromClass` "/Game/TopDown/Blueprints/BP_TopDownCharacter.BP_TopDownCharacter_C" (`self.GetTransform` (`self.Element`)) "Undefined" "MultiplyWithRoot" null null))
        (`Controller.Possess` _returnvalue _returnvalue_5)
        (bind _aspc_player_copie_2 (cast `/Game/Luminaria/Config/PC_Player_Copie` _returnvalue))
        (`KismetArrayLibrary.Array_Add` (`self.PlayerControllers`) _aspc_player_copie_2))))
  ;[0.02555 0 1] Init players controllers
  (for _array_element_2 (`self.PlayerControllers`)
    (`/Game/Luminaria/Config/PC_Player_Copie.Init` _array_element_2)))

(fn `UserConstructionScript`)