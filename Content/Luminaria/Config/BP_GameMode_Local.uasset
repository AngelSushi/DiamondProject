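; Local multiplayer game mode that creates and spawns one local player for each PlayerStart in the level on BeginPlay.
; Each player is created with the PlayerStart's index as controller ID and gets the IMC_Player Enhanced Input mapping context.
; The first player possesses a spawned BP_TopDownCharacter, while every later player possesses a BP_Fille at its own start.
; An older, disconnected BP_Player spawn path remains unused.
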(event `self.ReceiveBeginPlay`
  (bind _outactors (`GameplayStatics.GetAllActorsOfClass` "/Script/Engine.PlayerStart"))
  (for (_array_element _array_index) _outactors
    (set `self.Index` _array_index)
    (set `self.Element` _array_element)
    (bind _returnvalue (`GameplayStatics.CreatePlayer` (`self.Index`)))
    (if (> (`self.Index`) 0)
      (message `EnhancedInputSubsystemInterface.AddMappingContext` (pcsubsystem `EnhancedInputLocalPlayerSubsystem` _returnvalue) "/Game/Luminaria/Inputs/IMC_Player.IMC_Player" 0 (struct))
      (bind _returnvalue_2 (`|SpawnActorFromClass` "/Game/TopDown/Blueprints/BP_Fille.BP_Fille_C" (`self.GetTransform` (`self.Element`)) "Undefined" "MultiplyWithRoot" null null))
      (`Controller.Possess` (`GameplayStatics.GetPlayerController` (`self.Index`)) _returnvalue_2)
      (else
        (message `EnhancedInputSubsystemInterface.AddMappingContext` (pcsubsystem `EnhancedInputLocalPlayerSubsystem` _returnvalue) "/Game/Luminaria/Inputs/IMC_Player.IMC_Player" 0 (struct))
        (bind _returnvalue_3 (`|SpawnActorFromClass` "/Game/TopDown/Blueprints/BP_TopDownCharacter.BP_TopDownCharacter_C" (`self.GetTransform` (`self.Element`)) "Undefined" "MultiplyWithRoot" null null))
        (`Controller.Possess` (`GameplayStatics.GetPlayerController` 0) _returnvalue_3)))))

(fn `UserConstructionScript`)