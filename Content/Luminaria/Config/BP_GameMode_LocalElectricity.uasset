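; Game mode for Luminaria's local multiplayer that sets up one local player per PlayerStart in the level on BeginPlay.
; Each player gets the IMC_Player input mapping and a BP_TopDownCharacter spawned at its start and possessed, with player 0 using the existing first controller.
; Controllers are cast to DiamondProjectPlayerController and collected in PlayerControllers.
; The final controller init loop is empty, and an older BP_Player/PC_Player spawn path is left disconnected.
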(event `self.ReceiveBeginPlay`
  (bind _returnvalue (`GameplayStatics.GetPlayerController` 0))
  (bind _returnvalue_2 (`GameplayStatics.GetPlayerController` (`self.Index`)))
  (bind _outactors (`GameplayStatics.GetAllActorsOfClass` "/Script/Engine.PlayerStart"))
  (for (_array_element _array_index) _outactors
    (set `self.Index` _array_index)
    (set `self.Element` _array_element)
    (bind _returnvalue_3 (`GameplayStatics.CreatePlayer` (`self.Index`)))
    (if (> (`self.Index`) 0)
      (message `EnhancedInputSubsystemInterface.AddMappingContext` (pcsubsystem `EnhancedInputLocalPlayerSubsystem` _returnvalue_3) "/Game/Luminaria/Inputs/IMC_Player.IMC_Player" 0 (struct))
      (bind _returnvalue_4 (`|SpawnActorFromClass` "/Game/TopDown/Blueprints/BP_TopDownCharacter.BP_TopDownCharacter_C" (`self.GetTransform` (`self.Element`)) "Undefined" "MultiplyWithRoot" null null))
      (`Controller.Possess` _returnvalue_2 _returnvalue_4)
      (bind _asdiamond_project_player_controller (cast `DiamondProjectPlayerController` _returnvalue_2))
      (`KismetArrayLibrary.Array_Add` (`self.PlayerControllers`) _asdiamond_project_player_controller)
      (else
        (message `EnhancedInputSubsystemInterface.AddMappingContext` (pcsubsystem `EnhancedInputLocalPlayerSubsystem` (`GameplayStatics.GetPlayerController` 0)) "/Game/Luminaria/Inputs/IMC_Player.IMC_Player" 0 (struct))
        (bind _returnvalue_5 (`|SpawnActorFromClass` "/Game/TopDown/Blueprints/BP_TopDownCharacter.BP_TopDownCharacter_C" (`self.GetTransform` (`self.Element`)) "Undefined" "MultiplyWithRoot" null null))
        (`Controller.Possess` _returnvalue _returnvalue_5)
        (bind _asdiamond_project_player_controller_2 (cast `DiamondProjectPlayerController` _returnvalue))
        (`KismetArrayLibrary.Array_Add` (`self.PlayerControllers`) _asdiamond_project_player_controller_2))))
  ;[0.02555 0 1] Init players controllers
  (for _ (`self.PlayerControllers`)
    _))

(fn `UserConstructionScript`)